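; Utility AI for a shop that picks one catalog item to offer for a player's request.
; InitAI loads item rows from a data table; ScoreItem computes a weighted sum of profile fit, price, weight, rarity, value and profit, with CriteriaCount switching off terms.
; ChooseItem keeps the top scorer, remembers its type and price for "Cheaper" requests, and returns Polish text.
; The displayed "Score" is actually BaseValue; SellerGoalMode and RandomStream are only stored.
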(event `/Game/0-Main/AI/Test2/BPI_ShopAI.InitAI`
  (params (ItemsDT :type "DataTable Object Reference") (CatalogRows :type "Array of Name (by ref)") (CriteriaCount :type Integer) (SellerGoalMode :type Byte) (PlayerProfile :type Byte) (RandomStream :type "RandomStream Structure"))
  (set `self.ItemsDT` ItemsDT)
  (set `self.CatalogRows` CatalogRows)
  (set `self.CriteriaCount` CriteriaCount)
  (set `self.SellerGoalMode` SellerGoalMode)
  (set `self.PlayerProfile` PlayerProfile)
  (set `self.RandomStream` RandomStream)
  (`KismetArrayLibrary.Array_Clear` (`self.CatalogItems`))
  (for _array_element (`self.CatalogRows`)
    (bind _returnvalue (`|GetDataTableRow` (`self.ItemsDT`) _array_element)
      (:`then`
        (`KismetArrayLibrary.Array_Add` (`self.CatalogItems`) _returnvalue))))
  (set `self.bHasLastChoice` false))

(fn `ChooseItem`
  (params (Request :type "/Game/0-Main/AI/Test2/E_ShopRequest Enum" :default "NewEnumerator0"))
  (returns (ResultText :type Text))
  (locals (BestScore :type "Float (double-precision)" :default -999999.0) (BestItem :type "/Game/0-Main/Data/Test2/S_ItemData Structure") (bHasBest :type Boolean))
  (bind (_itemid _name _type _price _weight _rarity _fitprofile _basevalue) (break `/Game/0-Main/Data/Test2/S_ItemData` (`local.BestItem`)))
  (set `local.BestScore` -999999.0)
  (set `local.bHasBest` false)
  (switch `/Game/0-Main/AI/Test2/E_ShopRequest` Request
    (:`NewEnumerator0`
      _)
    (:`NewEnumerator1`
      _)
    (:`NewEnumerator2`
      _)
    (:`NewEnumerator3`
      _)
    (:`NewEnumerator4`
      _)
    (:`NewEnumerator5`
      (return "Wyjdż")))
  (for _array_element (`self.CatalogItems`)
    (bind _score (`self.ScoreItem` _array_element Request))
    (if (< (`local.BestScore`) _score)
      (set `local.BestScore` _score)
      (set `local.BestItem` _array_element)
      (set `local.bHasBest` true)))
  (if (`local.bHasBest`)
    (set `self.LastChosenType` _type)
    (set `self.LastChosenPrice` (`KismetMathLibrary.Conv_IntToDouble` _price))
    (set `self.bHasLastChoice` true)
    (return (`|FormatText` "[{ItemID}] {Name} | Type={Type} | Cena={Price} | Waga={Weight} | R={Rarity} | Fit={FitProfile} | Score={BestScore}" _itemid _name (`KismetMathLibrary.Conv_ByteToInt` _type) _price _weight _rarity _fitprofile _basevalue))
    (else
      (return "Brak pasujących przedmiotów"))))

(fn `ScoreItem`
  (params (Item :type "/Game/0-Main/Data/Test2/S_ItemData Structure") (Request :type "/Game/0-Main/AI/Test2/E_ShopRequest Enum" :default "NewEnumerator0"))
  (returns (Score :type "Float (double-precision)"))
  (locals (W_Fit :type "Float (double-precision)" :default 30.0) (W_Price :type "Float (double-precision)" :default 0.02) (W_Weight :type "Float (double-precision)" :default 1.5) (W_Rarity :type "Float (double-precision)" :default 8.0) (W_Base :type "Float (double-precision)" :default 0.02) (W_Profit :type "Float (double-precision)" :default 0.02) (TypeBonus :type "Float (double-precision)") (PriceMult :type "Float (double-precision)" :default 1.0) (DesiredType :type Integer :default -1))
  (bind (_itemid _name _type _price _weight _rarity _fitprofile _basevalue) (break `/Game/0-Main/Data/Test2/S_ItemData` Item))
  (bind _desiredtype (`local.DesiredType`))
  (set `local.TypeBonus` 0.0)
  (set `local.PriceMult` 1.0)
  (if (== (`self.CriteriaCount`) 2)
    (set `local.W_Weight` 0.0)
    (set `local.W_Rarity` 0.0)
    (set `local.W_Base` 0.0)
    (set `local.W_Profit` 0.0)
    (elif (== (`self.CriteriaCount`) 4)
      (set `local.W_Base` 0.0)
      (set `local.W_Profit` 0.0)))
  (switch `/Game/0-Main/AI/Test2/E_ShopRequest` Request
    (:`NewEnumerator0`
      (set `local.TypeBonus` (`KismetMathLibrary.SelectFloat` 50.0 0.0 (`|EnumEquality` _type "NewEnumerator0")))
      (set `local.DesiredType` 0))
    (:`NewEnumerator1`
      (set `local.TypeBonus` (`KismetMathLibrary.SelectFloat` 50.0 0.0 (`|EnumEquality` _type "NewEnumerator1")))
      (set `local.DesiredType` 1))
    (:`NewEnumerator2`
      (set `local.TypeBonus` (`KismetMathLibrary.SelectFloat` 50.0 0.0 (`|EnumEquality` _type "NewEnumerator2")))
      (set `local.DesiredType` 2))
    (:`NewEnumerator3`
      (set `local.TypeBonus` (`KismetMathLibrary.SelectFloat` 50.0 0.0 (`|EnumEquality` _type "NewEnumerator3")))
      (set `local.DesiredType` 3))
    (:`NewEnumerator4`
      (if (`self.bHasLastChoice`)
        (if (and (`|EnumEquality` _type (`self.LastChosenType`)) (< _price (`self.LastChosenPrice`)))
          (set `local.TypeBonus` 0.0)
          (set `local.PriceMult` 20.0)
          (set `local.DesiredType` -1)
          (else
            (`KismetSystemLibrary.PrintText` null "Nie ma tańszych przedmiotów")
            (return -999999.0)))
        (else
          (`KismetSystemLibrary.PrintText` null "Najpierw wybierz kategorię")
          (return -999999.0))))
    (:`NewEnumerator5`
      (return -999999.0)))
  (if (or (== _desiredtype (`KismetMathLibrary.Conv_ByteToInt` _type)) (== _desiredtype -1))
    (return (+ (`local.TypeBonus`) (* (`KismetMathLibrary.SelectFloat` 1.0 0.0 (== (`KismetMathLibrary.Conv_ByteToInt` _fitprofile) (`KismetMathLibrary.Conv_ByteToInt` (`self.PlayerProfile`)))) (`local.W_Fit`)) (* (* _price -1) (`local.W_Price`) (`local.PriceMult`)) (* _weight (`local.W_Weight`) -1.0) (* (`KismetMathLibrary.Conv_ByteToInt` _rarity) (`local.W_Rarity`)) (* _basevalue (`local.W_Base`)) (* (- _basevalue _price) (`local.W_Profit`))))
    (else
      (return -999999.0))))