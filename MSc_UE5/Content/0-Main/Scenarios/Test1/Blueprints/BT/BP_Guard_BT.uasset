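; BP_Guard_BT is the Behavior Tree variant of a guard AI in the Test1 scenario.
; StartGuardAI overrides a parent function, sets GuardActive, runs BT_Guard on the guard's AIController and prints debug messages, without calling the parent version.
; The EndGuardAI event stops the controller's brain component logic.
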(event `self.EndGuardAI`
  (bind _asaicontroller (cast `AIController` (`self.GetController`)))
  (`BrainComponent.StopLogic` (`AIController.BrainComponent` _asaicontroller) ""))

(fn `StartGuardAI`
  (`KismetSystemLibrary.PrintString` "BT GUARD AI STARTED")
  (set `self.bGuardActive` true)
  (bind _asaicontroller (cast `AIController` (`self.GetController`))
    (:`then`
      (`KismetSystemLibrary.PrintString` "BT: AIController OK")
      (`AIController.RunBehaviorTree` _asaicontroller "/Game/0-Main/Scenarios/Test1/Blueprints/BT/BT_Guard.BT_Guard"))
    (:`CastFailed`
      (`KismetSystemLibrary.PrintString` "BT: no AIController"))))

(fn `UserConstructionScript`
  (`parent.UserConstructionScript`))