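; Base guard AI for a test scenario that hunts the players and notifies the test controller when all are found.
; A looping timer runs GuardThink, which captures players within range, then uses AIMoveTo to chase seen players, investigate heard or last-known locations, or cycle through BP_SearchPoint actors.
; Sensing is hand-built from distance checks and a visibility trace for sight, with selectable sight, hearing or combined modes.
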(event `GuardThink`
  (if (`self.bGuardActive`)
    (`self.CheckCapture`)
    (if (>= (`KismetArrayLibrary.Array_Length` (`self.FoundPlayers`)) (`KismetArrayLibrary.Array_Length` (`self.Players`)))
      (`self.EndGuardAI`)
      (else
        (`self.DecideGuardAction`)
        (bind (_found_ _player_ _location _sensetype) (`self.SenseBestPlayer`))
        (if _found_
          (switch `/Game/0-Main/Scenarios/Test1/Blueprints/E_GuardSenseType` _sensetype
            (:`NewEnumerator1`
              (`self.StartChasePlayer` _player_))
            (:`NewEnumerator2`
              (`self.StartInvestigateLocation` _location _player_)))
          (elif (`self.bIsMovingToTarget`)
            _
            (elif (`self.bHasLastKnownLocation`)
              (`self.StartInvestigateLocation` (`self.LastKnownLocation`) (`self.CurrentTarget`))
              (else
                (bind (_found _location_2) (`self.GetNextSearchPoint`))
                (if _found
                  (`self.StartMoveToSearchPoint` _location_2))))))))))

(event `EndGuardAI`
  (bind _testcontroller (`self.TestController`))
  (set `self.bGuardActive` false)
  (`KismetSystemLibrary.K2_ClearAndInvalidateTimerHandle` (`self.GuardThinkTimerHandle`))
  (`KismetSystemLibrary.PrintString` "ALL PLAYERS FOUND")
  (if (`KismetSystemLibrary.IsValid` _testcontroller)
    (`/Game/0-Main/Scenarios/Test1/Blueprints/BP_Test1_Controller.FinishGuardPhase` _testcontroller)))

(event `StartMoveToSearchPoint`
  (params (Destination :type "Vector Structure"))
  (set `self.CurrentMoveMode` "NewEnumerator1")
  (set `self.bIsMovingToTarget` true)
  (bind _movementresult (`|AIMoveTo` self Destination null (`self.MoveAcceptanceRadius`))
    (:`OnSuccess`
      (`KismetSystemLibrary.PrintString` "Search point reached")
      (set `self.bIsMovingToTarget` false)
      (set `self.CurrentMoveMode` "NewEnumerator0"))
    (:`OnFail`
      (`KismetSystemLibrary.PrintString` "Search point move fail")
      (`KismetSystemLibrary.PrintString` (`|GetEnumeratorNameAsString` _movementresult))
      (set `self.bIsMovingToTarget` false)
      (set `self.CurrentMoveMode` "NewEnumerator0"))))

(event `StartInvestigateLocation`
  (params (Destination :type "Vector Structure") (Player :type "/Game/TopDown/Blueprints/BP_TopDownCharacter Object Reference"))
  (set `self.CurrentMoveMode` "NewEnumerator2")
  (set `self.CurrentTarget` Player)
  (set `self.LastKnownLocation` Destination)
  (set `self.bHasLastKnownLocation` true)
  (set `self.bIsMovingToTarget` true)
  (bind _movementresult (`|AIMoveTo` self Destination null (`self.MoveAcceptanceRadius`))
    (:`OnSuccess`
      (`KismetSystemLibrary.PrintString` "Investigate success")
      (set `self.bIsMovingToTarget` false)
      (set `self.CurrentMoveMode` "NewEnumerator0")
      (set `self.bHasLastKnownLocation` false)
      (`self.CheckCapture`))
    (:`OnFail`
      (`KismetSystemLibrary.PrintString` "Investigate fail")
      (`KismetSystemLibrary.PrintString` (`|GetEnumeratorNameAsString` _movementresult))
      (set `self.bIsMovingToTarget` false)
      (set `self.CurrentMoveMode` "NewEnumerator0"))))

(event `StartChasePlayer`
  (params (Player :type "/Game/TopDown/Blueprints/BP_TopDownCharacter Object Reference"))
  (set `self.CurrentMoveMode` "NewEnumerator3")
  (bind _output_get (set `self.CurrentTarget` Player))
  (set `self.LastKnownLocation` (`self.K2_GetActorLocation` Player))
  (set `self.bIsMovingToTarget` true)
  (bind _movementresult (`|AIMoveTo` self (0.0 0.0 0.0) Player (`self.MoveAcceptanceRadius`))
    (:`OnSuccess`
      (`KismetSystemLibrary.PrintString` "Chase success")
      (`self.MarkPlayerAsFound` _output_get)
      (set `self.bIsMovingToTarget` false)
      (`self.CheckCapture`))
    (:`OnFail`
      (`KismetSystemLibrary.PrintString` "Chase fail")
      (`KismetSystemLibrary.PrintString` (`|GetEnumeratorNameAsString` _movementresult))
      (set `self.bIsMovingToTarget` false)
      (set `self.CurrentMoveMode` "NewEnumerator0"))))

(fn `CanHearPlayer`
  (params (Player :type "/Game/TopDown/Blueprints/BP_TopDownCharacter Object Reference"))
  (returns (CanHear :type Boolean))
  (bind _hearingradius (`self.HearingRadius`))
  (bind _returnvalue (`KismetMathLibrary.Vector_Distance` (`self.K2_GetActorLocation`) (`self.K2_GetActorLocation` Player)))
  (bind _returnvalue_2 (<= _returnvalue _hearingradius))
  (if (`KismetSystemLibrary.IsValid` Player)
    (`KismetSystemLibrary.PrintString` (`KismetTextLibrary.Conv_TextToString` (`|FormatText` "Dist={Distance} HR={HearingRadius} Hear={CanHear}" _returnvalue _hearingradius _returnvalue_2)))
    (return _returnvalue_2)
    (else
      (`KismetSystemLibrary.PrintString` "error hearing")
      (return false))))

(fn `CanSeePlayer`
  (params (Player :type "/Game/TopDown/Blueprints/BP_TopDownCharacter Object Reference"))
  (returns (CanSee :type Boolean))
  (locals (start :type "Vector Structure") (end :type "Vector Structure"))
  (bind _returnvalue (`KismetMathLibrary.Vector_Distance` (`self.K2_GetActorLocation`) (`self.K2_GetActorLocation` Player)))
  (bind _returnvalue_2 (<= _returnvalue (`self.SightRadius`)))
  (if (`KismetSystemLibrary.IsValid` Player)
    (`KismetSystemLibrary.PrintText` (`|FormatText` "Dist={Distance} SR={SeeRadius} See={CanSee}" _returnvalue (`self.SightRadius`) _returnvalue_2))
    (if _returnvalue_2
      (set `local.start` (+ (`self.K2_GetActorLocation`) (0.0 0.0 80.0)))
      (set `local.end` (+ (`self.K2_GetActorLocation` Player) (0.0 0.0 80.0)))
      (bind _outhit (`KismetSystemLibrary.LineTraceSingle` (`local.start`) (`local.end`) "TraceTypeQuery1"))
      (if (== (`.HitActor` (`GameplayStatics.BreakHitResult` _outhit)) Player)
        (return true)
        (else
          (return false)))
      (else
        _))
    (else
      (`KismetSystemLibrary.PrintString` "error seeing")))
  (return false))

(fn `CheckCapture`
  (for _array_element (`self.Players`)
    (if (`KismetSystemLibrary.IsValid` _array_element)
      (bind _isfound (`self.IsPlayerFound` _array_element))
      (if _isfound
        _
        (elif (<= (`KismetMathLibrary.Vector_Distance` (`self.K2_GetActorLocation`) (`self.K2_GetActorLocation` _array_element)) (`self.CaptureRadius`))
          (`self.MarkPlayerAsFound` _array_element)
          (`KismetSystemLibrary.PrintString` "Player Found")))))
  (if (>= (`KismetArrayLibrary.Array_Length` (`self.FoundPlayers`)) (`KismetArrayLibrary.Array_Length` (`self.Players`)))
    (`self.EndGuardAI`)))

(fn `DecideGuardAction`)

(fn `GetNearestUnfoundPlayer`
  (returns (Player :type "/Game/TopDown/Blueprints/BP_TopDownCharacter Object Reference") (Found :type Boolean) (Distance :type "Float (double-precision)") (Location :type "Vector Structure"))
  (locals (BestPlayer :type "/Game/TopDown/Blueprints/BP_TopDownCharacter Object Reference") (BestDistance :type "Float (double-precision)") (FoundLocal :type Boolean))
  (bind _bestplayer (`local.BestPlayer`))
  (set `local.FoundLocal` false)
  (set `local.BestDistance` 99999999.0)
  (for _array_element (`self.Players`)
    (if (`KismetSystemLibrary.IsValid` _array_element)
      (if (not (`KismetArrayLibrary.Array_Contains` (`self.FoundPlayers`) _array_element))
        (bind _returnvalue (`KismetMathLibrary.Vector_Distance` (`self.K2_GetActorLocation`) (`self.K2_GetActorLocation` _array_element)))
        (if (< _returnvalue (`local.BestDistance`))
          (set `local.BestDistance` _returnvalue)
          (set `local.BestPlayer` _array_element)
          (set `local.FoundLocal` true)))))
  (return _bestplayer (`local.FoundLocal`) (`local.BestDistance`) (`self.K2_GetActorLocation` _bestplayer)))

(fn `GetNextSearchPoint`
  (returns (Found :type Boolean) (Location :type "Vector Structure"))
  (bind _searchpoints (`self.SearchPoints`))
  (bind _currentsearchindex (`self.CurrentSearchIndex`))
  (bind _returnvalue (`KismetArrayLibrary.Array_Length` _searchpoints))
  (bind _output (`|GetArrayItem` _searchpoints _currentsearchindex))
  (if (> _returnvalue 0)
    (set `self.CurrentSearchIndex` (+ (`self.CurrentSearchIndex`) 1))
    (if (>= _currentsearchindex _returnvalue)
      (set `self.CurrentSearchIndex` 0))
    (if (`KismetSystemLibrary.IsValid` _output)
      (return true (`self.K2_GetActorLocation` _output))
      (else
        (return false (`self.K2_GetActorLocation`))))
    (else
      (return false (`self.K2_GetActorLocation`)))))

(fn `InitGuard`
  (params (PlayersIn :type "Array of /Game/TopDown/Blueprints/BP_TopDownCharacter Object Reference") (ControllerIn :type "/Game/0-Main/Scenarios/Test1/Blueprints/BP_Test1_Controller Object Reference") (SenseModeIn :type "/Game/0-Main/Scenarios/Test1/Blueprints/E_GuardSenseMode Enum" :default "NewEnumerator0"))
  (bind _output_get (set `self.Players` PlayersIn))
  (for _array_element _output_get
    (if (`KismetSystemLibrary.IsValid` _array_element)
      (`KismetSystemLibrary.PrintString` "VALID PLAYER")
      (else
        (`KismetSystemLibrary.PrintString` "NOT VALID PLAYER"))))
  (set `self.TestController` ControllerIn)
  (`KismetArrayLibrary.Array_Clear` (`self.FoundPlayers`))
  (set `self.CurrentTarget` null)
  (set `self.bHasLastKnownLocation` false)
  (set `self.SenseMode` SenseModeIn)
  (bind _outactors (`GameplayStatics.GetAllActorsOfClass` "/Game/0-Main/Scenarios/Test1/Blueprints/BP_SearchPoint.BP_SearchPoint_C"))
  (bind _output_get_2 (set `self.SearchPoints` _outactors))
  (`KismetSystemLibrary.PrintString` (`KismetStringLibrary.Conv_IntToString` (`KismetArrayLibrary.Array_Length` _output_get_2)))
  (return))

(fn `IsPlayerFound`
  (params (Player :type "/Game/TopDown/Blueprints/BP_TopDownCharacter Object Reference"))
  (returns (isFound :type Boolean))
  (return (`KismetArrayLibrary.Array_Contains` (`self.FoundPlayers`) Player)))

(fn `MarkPlayerAsFound`
  (params (Player :type "/Game/TopDown/Blueprints/BP_TopDownCharacter Object Reference"))
  (`KismetSystemLibrary.PrintString` "MARK PLAYER CALLED")
  (if (`KismetSystemLibrary.IsValid` Player)
    (if (not (`KismetArrayLibrary.Array_Contains` (`self.FoundPlayers`) Player))
      (`KismetArrayLibrary.Array_AddUnique` (`self.FoundPlayers`) Player))
    (if (== (`self.CurrentTarget`) Player)
      (set `self.CurrentTarget` null)
      (set `self.bHasLastKnownLocation` false)
      (set `self.LastKnownLocation` (0.0 0.0 0.0))
      (set `self.bIsMovingToTarget` false)
      (set `self.CurrentMoveMode` "NewEnumerator0")
      (`CharacterMovementComponent.DisableMovement` (`Character.CharacterMovement` Player))
      (`self.SetActorEnableCollision` Player false))
    (else
      (return))))

(fn `SenseBestPlayer`
  (returns (`Found ` :type Boolean) (`Player ` :type "/Game/TopDown/Blueprints/BP_TopDownCharacter Object Reference") (Location :type "Vector Structure") (SenseType :type "/Game/0-Main/Scenarios/Test1/Blueprints/E_GuardSenseType Enum"))
  (locals (FoundLocal :type Boolean))
  (for _array_element (`self.Players`)
    (if (`KismetSystemLibrary.IsValid` _array_element)
      (bind _isfound (`self.IsPlayerFound` _array_element))
      (if (not _isfound)
        (switch `/Game/0-Main/Scenarios/Test1/Blueprints/E_GuardSenseMode` (`self.SenseMode`)
          (:`NewEnumerator0`
            (bind _cansee (`self.CanSeePlayer` _array_element))
            (if _cansee
              (set `self.CurrentTarget` _array_element)
              (bind _returnvalue (`self.K2_GetActorLocation` _array_element))
              (set `self.LastKnownLocation` _returnvalue)
              (set `self.bHasLastKnownLocation` true)
              (return true _array_element _returnvalue "NewEnumerator1")
              (else
                (bind _canhear (`self.CanHearPlayer` _array_element))
                (if _canhear
                  (set `self.CurrentTarget` null)
                  (bind _returnvalue_2 (`self.K2_GetActorLocation` _array_element))
                  (set `self.LastKnownLocation` _returnvalue_2)
                  (set `self.bHasLastKnownLocation` true)
                  (return true _array_element _returnvalue_2 "NewEnumerator2")))))
          (:`NewEnumerator1`
            (bind _cansee_2 (`self.CanSeePlayer` _array_element))
            (if _cansee_2
              (set `self.CurrentTarget` _array_element)
              (bind _returnvalue_3 (`self.K2_GetActorLocation` _array_element))
              (set `self.LastKnownLocation` _returnvalue_3)
              (set `self.bHasLastKnownLocation` true)
              (return true _array_element _returnvalue_3 "NewEnumerator1")))
          (:`NewEnumerator2`
            (bind _canhear_2 (`self.CanHearPlayer` _array_element))
            (if _canhear_2
              (set `self.CurrentTarget` _array_element)
              (bind _returnvalue_4 (`self.K2_GetActorLocation` _array_element))
              (set `self.LastKnownLocation` _returnvalue_4)
              (set `self.bHasLastKnownLocation` true)
              (return true _array_element _returnvalue_4 "NewEnumerator2"))))))))

(fn `StartGuardAI`
  (`KismetSystemLibrary.PrintString` "GUARD AI STARTED")
  (set `self.bGuardActive` true)
  (bind _returnvalue (`KismetSystemLibrary.K2_SetTimerDelegate` (`|CreateDelegate` :!event `GuardThink`) (`self.ThinkInterval`) true))
  (set `self.GuardThinkTimerHandle` _returnvalue)
  (`self.GuardThink`))

(fn `StopCurrentMove`
  (bind _asaicontroller (cast `AIController` (`self.GetController`)))
  (`Controller.StopMovement` _asaicontroller)
  (set `self.bIsMovingToTarget` false)
  (set `self.CurrentMoveMode` "NewEnumerator0"))

(fn `UserConstructionScript`)