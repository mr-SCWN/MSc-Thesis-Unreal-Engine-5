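; Controller for the Test1 scenario, running a timed player escape phase followed by an AI guard phase.
; StartScenario reads the config, spawns players in a row at PlayerStart, and a looping timer hands possession to each in turn, freezing the previous one.
; After the last turn it spawns a guard with the player list and configured sense mode.
; FinishGuardPhase sends the stop message, though StopScenario itself is empty.
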(event `/Game/0-Main/Core/Interfaces/BPI_TestScenario.StartScenario`
  (params (TestConfig :type "/Game/0-Main/Core/Configs/DA_TestConfig Object Reference"))
  (bind (_test1_escapetimen _test1_playerscount _test1_searchtimelimittmax) (break `/Game/0-Main/Core/Structs/S_Test1Settings` (`/Game/0-Main/Core/Configs/DA_TestConfig.Test1` (`self.ConfigRef`))))
  (set `self.ConfigRef` TestConfig)
  (set `self.PlayersCount` _test1_playerscount)
  (set `self.SearchTimeLimitMax` _test1_searchtimelimittmax)
  (set `self.EscapeTimeN` _test1_escapetimen)
  (set `self.ActiveIndex` 0)
  (`KismetArrayLibrary.Array_Clear` (`self.SpawnedPlayers`))
  (bind _returnvalue (`GameplayStatics.GetActorOfClass` "/Script/Engine.PlayerStart"))
  (for _index (range (`self.PlayersCount`))
    (bind _returnvalue_2 (`|SpawnActorFromClass` (`self.PlayerClass`) (`KismetMathLibrary.MakeTransform` (+ (`self.K2_GetActorLocation` _returnvalue) (`KismetMathLibrary.MakeVector` 0.0 (* _index 200.0))) (`self.K2_GetActorRotation` _returnvalue)) "Undefined" "MultiplyWithRoot" null null))
    (`KismetArrayLibrary.Array_Add` (`self.SpawnedPlayers`) _returnvalue_2))
  (`Controller.Possess` (`GameplayStatics.GetPlayerController` 0) (`|GetArrayItem` (`self.SpawnedPlayers`)))
  (bind _returnvalue_3 (`KismetSystemLibrary.K2_SetTimerDelegate` (`|CreateDelegate` :!event `SwitchToNextPlayer`) (`self.EscapeTimeN`) true))
  (set `self.SwitchTimerHandle` _returnvalue_3))

(event `SwitchToNextPlayer`
  (bind _output (`|GetArrayItem` (`self.SpawnedPlayers`) (`self.ActiveIndex`)))
  (bind _charactermovement (`Character.CharacterMovement` (`|GetArrayItem` (`self.SpawnedPlayers`) (`self.ActiveIndex`))))
  (`MovementComponent.StopMovementImmediately` _charactermovement)
  (`CharacterMovementComponent.DisableMovement` _charactermovement)
  (set `self.ActiveIndex` (+ (`self.ActiveIndex`) 1))
  (if (< (`self.ActiveIndex`) (`self.PlayersCount`))
    (`Controller.Possess` (`GameplayStatics.GetPlayerController` 0) _output)
    (`CharacterMovementComponent.SetMovementMode` (`Character.CharacterMovement` _output) "MOVE_Walking" 0)
    (else
      (`KismetSystemLibrary.K2_ClearAndInvalidateTimerHandle` (`self.SwitchTimerHandle`))
      (`self.StartGuardPhase`))))

(event `/Game/0-Main/Core/Interfaces/BPI_TestScenario.StopScenario`)

(event `StartGuardPhase`
  (bind _spawnedplayers (`self.SpawnedPlayers`))
  (bind _returnvalue (`GameplayStatics.GetActorOfClass` "/Script/Engine.PlayerStart"))
  (bind _returnvalue_2 (`|SpawnActorFromClass` (`self.GuardClass`) (`KismetMathLibrary.MakeTransform` (`self.K2_GetActorLocation` _returnvalue) (`self.K2_GetActorRotation` _returnvalue)) "Undefined" "MultiplyWithRoot" null null))
  (bind _output_get (set `self.SpawnedGuard` _returnvalue_2))
  (`KismetSystemLibrary.PrintString` "\"Players before guard init: \"")
  (`KismetSystemLibrary.PrintString` (`KismetStringLibrary.Conv_IntToString` (`KismetArrayLibrary.Array_Length` _spawnedplayers)))
  (`Pawn.SpawnDefaultController` _output_get)
  (`/Game/0-Main/Scenarios/Test1/Blueprints/BP_Guard_Base.InitGuard` _output_get _spawnedplayers self (`.GuardSenseMode_11_A6C5AC3246619352A0DD9883FACB6A82` (break `/Game/0-Main/Core/Structs/S_Test1Settings` (`/Game/0-Main/Core/Configs/DA_TestConfig.Test1` (`self.ConfigRef`)))))
  (`/Game/0-Main/Scenarios/Test1/Blueprints/BP_Guard_Base.StartGuardAI` _output_get))

(event `FinishGuardPhase`
  (`KismetSystemLibrary.PrintString` "TEST1 GUARD PHASE FINISHED")
  (message `/Game/0-Main/Core/Interfaces/BPI_TestScenario.StopScenario` self))

(fn `GetScenarioName`
  (returns (GetScenarioName :type String))
  (return ""))

(fn `UserConstructionScript`)