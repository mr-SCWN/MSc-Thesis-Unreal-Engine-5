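; Utility AI guard Blueprint that overrides DecideGuardAction to choose between chasing, investigating and searching.
; When idle, it scores one candidate from sight, hearing, last known location or next search point, adding a clamped linear distance bonus for sensed players.
; While moving, sight or hearing interrupts the current move depending on move mode.
; The sight score compares against itself, so idle guards never start a chase.
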(fn `DecideGuardAction`
  (locals (BestAction :type "/Game/0-Main/Scenarios/Test1/Blueprints/E_GuardUAIAction Enum") (BestScore :type "Float (double-precision)" :default -9999.0) (CandidateScore :type "Float (double-precision)") (SensedFound :type Boolean) (SensedPlayer :type "/Game/TopDown/Blueprints/BP_TopDownCharacter Object Reference") (SensedLocation :type "Vector Structure") (SensedType :type "/Game/0-Main/Scenarios/Test1/Blueprints/E_GuardSenseType Enum") (DistanceToPlayer :type "Float (double-precision)") (SearchFound :type Boolean) (SearchLocation :type "Vector Structure") (BestPlayer :type "/Game/TopDown/Blueprints/BP_TopDownCharacter Object Reference") (BestLocation :type "Vector Structure"))
  (set `local.BestAction` "NewEnumerator0")
  (set `local.BestScore` -9999.0)
  (bind (_found_ _player_ _location _sensetype) (`self.SenseBestPlayer`))
  (set `local.SensedFound` _found_)
  (set `local.SensedPlayer` _player_)
  (set `local.SensedLocation` _location)
  (bind _output_get (set `local.SensedType` _sensetype))
  (if (`self.bIsMovingToTarget`)
    (if (`local.SensedFound`)
      (switch `/Game/0-Main/Scenarios/Test1/Blueprints/E_GuardSenseType` _output_get
        (:`NewEnumerator1`
          (if (`|EnumInequality` (`self.CurrentMoveMode`) "NewEnumerator3")
            (`self.StopCurrentMove`)
            (`self.StartChasePlayer` (`local.SensedPlayer`))
            (return)
            (else
              (return))))
        (:`NewEnumerator2`
          (if (`|EnumEquality` (`self.CurrentMoveMode`) "NewEnumerator1")
            (`self.StopCurrentMove`)
            (`self.StartInvestigateLocation` (`local.SensedLocation`) (`local.SensedPlayer`))
            (return)
            (else
              (return))))))
    (else
      ; Utility AI Logic
      (if (`local.SensedFound`)
        (switch `/Game/0-Main/Scenarios/Test1/Blueprints/E_GuardSenseType` (`local.SensedType`)
          (:`NewEnumerator1`
            (bind _bonus (`self.UAI_CalculateDistanceBonus` (`KismetMathLibrary.Vector_Distance` (`self.K2_GetActorLocation`) (`self.K2_GetActorLocation` (`local.SensedPlayer`))) (`self.SightRadius`)))
            (bind _output_get_2 (set `local.CandidateScore` (+ (`self.UAI_Score_Sight`) _bonus)))
            (if (> _output_get_2 (`local.CandidateScore`))
              (set `local.BestScore` (`local.CandidateScore`))
              (set `local.BestAction` "NewEnumerator3")
              (set `local.BestPlayer` (`local.SensedPlayer`))
              (set `local.BestLocation` (`local.SensedLocation`))
              (switch `/Game/0-Main/Scenarios/Test1/Blueprints/E_GuardUAIAction` (`local.BestAction`) :!label _label
                (:`NewEnumerator0`
                  (`KismetSystemLibrary.PrintString` " UAI: None"))
                (:`NewEnumerator1`
                  (`KismetSystemLibrary.PrintString` " UAI: Search")
                  (`self.StartMoveToSearchPoint` (`local.BestLocation`))
                  (return))
                (:`NewEnumerator2`
                  (`KismetSystemLibrary.PrintString` " UAI: Investigate")
                  (`self.StartInvestigateLocation` (`local.BestLocation`) (`local.BestPlayer`))
                  (return))
                (:`NewEnumerator3`
                  (`KismetSystemLibrary.PrintString` " UAI: Chase")
                  (`self.StartChasePlayer` (`local.BestPlayer`))
                  (return)))))
          (:`NewEnumerator2`
            (bind _bonus_2 (`self.UAI_CalculateDistanceBonus` (`KismetMathLibrary.Vector_Distance` (`self.K2_GetActorLocation`) (`self.K2_GetActorLocation` (`local.SensedPlayer`))) (`self.HearingRadius`)))
            (bind _output_get_3 (set `local.CandidateScore` (+ _bonus_2 (`self.UAI_Score_Hearing`))))
            (if (> _output_get_3 (`local.BestScore`))
              (set `local.BestScore` (`local.CandidateScore`))
              (set `local.BestAction` "NewEnumerator2")
              (set `local.BestPlayer` (`local.SensedPlayer`))
              (set `local.BestLocation` (`local.SensedLocation`))
              (goto _label))))
        (elif (`self.bHasLastKnownLocation`)
          (bind _output_get_4 (set `local.CandidateScore` (`self.UAI_Score_LastKnownLocation`)))
          (if (> _output_get_4 (`local.BestScore`))
            (set `local.BestScore` (`local.CandidateScore`))
            (set `local.BestAction` "NewEnumerator2")
            (set `local.BestPlayer` (`self.CurrentTarget`))
            (set `local.BestLocation` (`self.LastKnownLocation`))
            (goto _label))
          (else
            (bind (_found _location_2) (`self.GetNextSearchPoint`))
            (set `local.SearchFound` _found)
            (set `local.SearchLocation` _location_2)
            (if (`local.SearchFound`)
              (bind _output_get_5 (set `local.CandidateScore` (`self.UAI_Score_Search`)))
              (if (> _output_get_5 (`local.BestScore`))
                (set `local.BestScore` (`local.CandidateScore`))
                (set `local.BestAction` "NewEnumerator1")
                (set `local.BestLocation` (`local.SearchLocation`))
                (goto _label)))))))))

(fn `UAI_CalculateDistanceBonus`
  (params (Distance :type "Float (double-precision)") (Radius :type "Float (double-precision)"))
  (returns (Bonus :type "Float (double-precision)"))
  (return (* (- 1.0 (`KismetMathLibrary.FClamp` (/ Distance Radius))) (`self.UAI_DistanceBonusMax`))))

(fn `UserConstructionScript`
  (`parent.UserConstructionScript`))