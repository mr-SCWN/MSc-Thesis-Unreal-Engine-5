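; StateTree task that decides whether the guard's AI run can finish in the Test1 scenario.
; On entering the state, it casts the actor to BP_Guard_ST and compares the found players count to the total players count.
; When all are found it calls EndGuardAI; otherwise it clears the search flag and resets the guard's current decision, printing a debug message either way.
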(event `self.ReceiveLatentEnterState`
  (params (Transition :type "StateTreeTransitionResult Structure (by ref)"))
  (bind _asbp_guard_st (cast `/Game/0-Main/Scenarios/Test1/Blueprints/ST/BP_Guard_ST` (`self.Actor`)))
  (if (>= (`KismetArrayLibrary.Array_Length` (`/Game/0-Main/Scenarios/Test1/Blueprints/BP_Guard_Base.FoundPlayers` _asbp_guard_st)) (`KismetArrayLibrary.Array_Length` (`/Game/0-Main/Scenarios/Test1/Blueprints/BP_Guard_Base.Players` _asbp_guard_st)))
    (`KismetSystemLibrary.PrintString` "ST STATE: FINISHED")
    (`/Game/0-Main/Scenarios/Test1/Blueprints/BP_Guard_Base.EndGuardAI` _asbp_guard_st)
    (else
      (`KismetSystemLibrary.PrintString` "ST FINISH BLOCKED: NOT ALL FOUND")
      (set `/Game/0-Main/Scenarios/Test1/Blueprints/ST/BP_Guard_ST.ST_WantsSearch` false _asbp_guard_st)
      (set `/Game/0-Main/Scenarios/Test1/Blueprints/ST/BP_Guard_ST.ST_CurrentDecision` "NewEnumerator1" _asbp_guard_st))))