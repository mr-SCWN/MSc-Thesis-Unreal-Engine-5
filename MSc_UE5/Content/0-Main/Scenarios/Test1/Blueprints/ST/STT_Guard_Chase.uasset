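; StateTree task that runs the chase state of BP_Guard_ST, a guard that hunts and captures players.
; On entry it restarts movement toward the current target, or requests a search if the target is invalid or already found.
; Each tick it checks for capture, requests finish once all players are found, and otherwise drops lost or found targets back to search.
; Transitions are signalled through flags and a decision enum on the guard.
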(event `self.ReceiveLatentEnterState`
  (params (Transition :type "StateTreeTransitionResult Structure (by ref)"))
  (bind _asbp_guard_st (cast `/Game/0-Main/Scenarios/Test1/Blueprints/ST/BP_Guard_ST` (`self.Actor`)))
  (`KismetSystemLibrary.PrintString` "ST STATE: CHASE")
  (bind _currenttarget (`/Game/0-Main/Scenarios/Test1/Blueprints/BP_Guard_Base.CurrentTarget` _asbp_guard_st))
  (if (`KismetSystemLibrary.IsValid` _currenttarget)
    (bind _isfound (`/Game/0-Main/Scenarios/Test1/Blueprints/BP_Guard_Base.IsPlayerFound` _asbp_guard_st _currenttarget))
    (if _isfound
      (set `/Game/0-Main/Scenarios/Test1/Blueprints/BP_Guard_Base.CurrentTarget` null _asbp_guard_st)
      (set `/Game/0-Main/Scenarios/Test1/Blueprints/BP_Guard_Base.bHasLastKnownLocation` false _asbp_guard_st)
      (set `/Game/0-Main/Scenarios/Test1/Blueprints/ST/BP_Guard_ST.ST_WantsSearch` true _asbp_guard_st)
      (set `/Game/0-Main/Scenarios/Test1/Blueprints/ST/BP_Guard_ST.ST_CurrentDecision` "NewEnumerator1" _asbp_guard_st)
      (else
        (if (`/Game/0-Main/Scenarios/Test1/Blueprints/BP_Guard_Base.bIsMovingToTarget` _asbp_guard_st)
          (`/Game/0-Main/Scenarios/Test1/Blueprints/BP_Guard_Base.StopCurrentMove` _asbp_guard_st))
        (`/Game/0-Main/Scenarios/Test1/Blueprints/BP_Guard_Base.StartChasePlayer` _asbp_guard_st _currenttarget)))
    (else
      (set `/Game/0-Main/Scenarios/Test1/Blueprints/ST/BP_Guard_ST.ST_WantsSearch` true _asbp_guard_st)
      (set `/Game/0-Main/Scenarios/Test1/Blueprints/ST/BP_Guard_ST.ST_CurrentDecision` "NewEnumerator1" _asbp_guard_st))))

(event `self.ReceiveLatentTick`
  (params (DeltaTime :type "Float (single-precision)"))
  (bind _asbp_guard_st (cast `/Game/0-Main/Scenarios/Test1/Blueprints/ST/BP_Guard_ST` (`self.Actor`)))
  (`/Game/0-Main/Scenarios/Test1/Blueprints/BP_Guard_Base.CheckCapture` _asbp_guard_st)
  (if (>= (`KismetArrayLibrary.Array_Length` (`/Game/0-Main/Scenarios/Test1/Blueprints/BP_Guard_Base.FoundPlayers` _asbp_guard_st)) (`KismetArrayLibrary.Array_Length` (`/Game/0-Main/Scenarios/Test1/Blueprints/BP_Guard_Base.Players` _asbp_guard_st)))
    (set `/Game/0-Main/Scenarios/Test1/Blueprints/ST/BP_Guard_ST.ST_WantsFinish` true _asbp_guard_st)
    (set `/Game/0-Main/Scenarios/Test1/Blueprints/ST/BP_Guard_ST.ST_CurrentDecision` "NewEnumerator4" _asbp_guard_st)
    (else
      (bind _currenttarget (`/Game/0-Main/Scenarios/Test1/Blueprints/BP_Guard_Base.CurrentTarget` _asbp_guard_st))
      (if (`KismetSystemLibrary.IsValid` _currenttarget)
        (bind _isfound (`/Game/0-Main/Scenarios/Test1/Blueprints/BP_Guard_Base.IsPlayerFound` _asbp_guard_st _currenttarget))
        (if _isfound
          (set `/Game/0-Main/Scenarios/Test1/Blueprints/BP_Guard_Base.CurrentTarget` null _asbp_guard_st)
          (set `/Game/0-Main/Scenarios/Test1/Blueprints/BP_Guard_Base.bHasLastKnownLocation` false _asbp_guard_st)
          (set `/Game/0-Main/Scenarios/Test1/Blueprints/BP_Guard_Base.LastKnownLocation` (0.0 0.0 0.0) _asbp_guard_st)
          (set `/Game/0-Main/Scenarios/Test1/Blueprints/ST/BP_Guard_ST.ST_WantsSearch` true _asbp_guard_st)
          (set `/Game/0-Main/Scenarios/Test1/Blueprints/ST/BP_Guard_ST.ST_CurrentDecision` "NewEnumerator1" _asbp_guard_st))
        (else
          (set `/Game/0-Main/Scenarios/Test1/Blueprints/BP_Guard_Base.bHasLastKnownLocation` false _asbp_guard_st)
          (set `/Game/0-Main/Scenarios/Test1/Blueprints/BP_Guard_Base.LastKnownLocation` (0.0 0.0 0.0) _asbp_guard_st)
          (set `/Game/0-Main/Scenarios/Test1/Blueprints/ST/BP_Guard_ST.ST_WantsSearch` true _asbp_guard_st)
          (set `/Game/0-Main/Scenarios/Test1/Blueprints/ST/BP_Guard_ST.ST_CurrentDecision` "NewEnumerator1" _asbp_guard_st))))))