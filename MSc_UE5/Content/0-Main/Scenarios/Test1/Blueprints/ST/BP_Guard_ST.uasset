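; BP_Guard_ST is a guard Blueprint variant whose AI runs on a StateTree to hunt players, with start and end hooks for that logic.
; STUpdateDecision checks capture and sensing, then sets search, investigate, chase or finish flags and a decision enum.
; Sight and hearing store target and last known location and set the chase flag, though hearing's enum matches investigate.
; StartGuardAI starts the StateTree without calling the parent version.
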(event `self.EndGuardAI`
  (`BrainComponent.StopLogic` (`self.StateTreeAI`) ""))

(fn `ST_ResetDecisionFlags`
  (set `self.ST_WantsSearch` false)
  (set `self.ST_WantsInvestigate` false)
  (set `self.ST_WantsChase` false)
  (set `self.ST_WantsFinish` false)
  (set `self.ST_CurrentDecision` "NewEnumerator0"))

(fn `ST_UpdateDecision`
  (`self.ST_ResetDecisionFlags`)
  (`self.CheckCapture`)
  (if (>= (`KismetArrayLibrary.Array_Length` (`self.FoundPlayers`)) (`KismetArrayLibrary.Array_Length` (`self.Players`)))
    (set `self.ST_WantsFinish` true)
    (set `self.ST_CurrentDecision` "NewEnumerator4")
    (else
      (bind (_found_ _player_ _location _sensetype) (`self.SenseBestPlayer`))
      (set `self.ST_SensedFound` _found_)
      (set `self.ST_SensedPlayer` _player_)
      (set `self.ST_SensedLocation` _location)
      (set `self.ST_SensedType` _sensetype)
      (if (`self.ST_SensedFound`)
        (bind _isfound (`self.IsPlayerFound` (`self.ST_SensedPlayer`)))
        (if _isfound
          (set `self.ST_WantsSearch` true)
          (set `self.ST_CurrentDecision` "NewEnumerator1")
          (`KismetSystemLibrary.PrintString` "ST DECISION: FINISHED")
          (else
            (switch `/Game/0-Main/Scenarios/Test1/Blueprints/E_GuardSenseType` (`self.ST_SensedType`)
              (:`NewEnumerator1`
                (set `self.CurrentTarget` (`self.ST_SensedPlayer`))
                (set `self.LastKnownLocation` (`self.ST_SensedLocation`))
                (set `self.bHasLastKnownLocation` true)
                (set `self.ST_WantsChase` true)
                (set `self.ST_CurrentDecision` "NewEnumerator3")
                (`KismetSystemLibrary.PrintString` "ST DECISION: CHASE"))
              (:`NewEnumerator2`
                (set `self.CurrentTarget` (`self.ST_SensedPlayer`))
                (set `self.LastKnownLocation` (`self.ST_SensedLocation`))
                (set `self.bHasLastKnownLocation` true)
                (set `self.ST_WantsChase` true)
                (set `self.ST_CurrentDecision` "NewEnumerator2")
                (`KismetSystemLibrary.PrintString` "ST DECISION: INVESTIGATE")))))
        (elif (`self.bHasLastKnownLocation`)
          (set `self.ST_WantsInvestigate` true)
          (set `self.ST_CurrentDecision` "NewEnumerator2")
          (`KismetSystemLibrary.PrintString` "ST DECISION: INVESTIGATE LAST KNOWN")
          (else
            (set `self.ST_WantsSearch` true)
            (set `self.ST_CurrentDecision` "NewEnumerator1")
            (`KismetSystemLibrary.PrintString` "ST DECISION: SEARCH")))))))

(fn `StartGuardAI`
  (`KismetSystemLibrary.PrintString` "ST GUARD AI STARTED")
  (set `self.bGuardActive` true)
  (`BrainComponent.StartLogic` (`self.StateTreeAI`)))

(fn `UserConstructionScript`
  (`parent.UserConstructionScript`))