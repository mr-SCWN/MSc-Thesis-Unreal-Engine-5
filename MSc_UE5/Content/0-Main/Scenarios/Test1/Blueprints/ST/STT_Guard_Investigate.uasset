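; StateTree task that runs a guard's Investigate state, sending it to the last known location of its current target.
; On enter it stops any active move, then calls StartInvestigateLocation on the BP_Guard_ST actor.
; Each tick, once the guard stops moving without wanting a chase, it clears the target and last-known-location flag.
; It then sets the search flag and updates the guard's decision enum, without finishing the task itself.
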(event `self.ReceiveLatentEnterState`
  (params (Transition :type "StateTreeTransitionResult Structure (by ref)"))
  (bind _asbp_guard_st (cast `/Game/0-Main/Scenarios/Test1/Blueprints/ST/BP_Guard_ST` (`self.Actor`)))
  (`KismetSystemLibrary.PrintString` "ST STATE: INVESTIGATE")
  (if (`/Game/0-Main/Scenarios/Test1/Blueprints/BP_Guard_Base.bIsMovingToTarget` _asbp_guard_st)
    (`/Game/0-Main/Scenarios/Test1/Blueprints/BP_Guard_Base.StopCurrentMove` _asbp_guard_st))
  (`/Game/0-Main/Scenarios/Test1/Blueprints/BP_Guard_Base.StartInvestigateLocation` _asbp_guard_st (`/Game/0-Main/Scenarios/Test1/Blueprints/BP_Guard_Base.LastKnownLocation` _asbp_guard_st) (`/Game/0-Main/Scenarios/Test1/Blueprints/BP_Guard_Base.CurrentTarget` _asbp_guard_st)))

(event `self.ReceiveLatentTick`
  (params (DeltaTime :type "Float (single-precision)"))
  (bind _asbp_guard_st (cast `/Game/0-Main/Scenarios/Test1/Blueprints/ST/BP_Guard_ST` (`self.Actor`)))
  (if (`/Game/0-Main/Scenarios/Test1/Blueprints/BP_Guard_Base.bIsMovingToTarget` _asbp_guard_st)
    _
    (elif (not (`/Game/0-Main/Scenarios/Test1/Blueprints/ST/BP_Guard_ST.ST_WantsChase` _asbp_guard_st))
      (set `/Game/0-Main/Scenarios/Test1/Blueprints/BP_Guard_Base.CurrentTarget` null _asbp_guard_st)
      (set `/Game/0-Main/Scenarios/Test1/Blueprints/BP_Guard_Base.bHasLastKnownLocation` false _asbp_guard_st)
      (set `/Game/0-Main/Scenarios/Test1/Blueprints/ST/BP_Guard_ST.ST_WantsSearch` true _asbp_guard_st)
      (set `/Game/0-Main/Scenarios/Test1/Blueprints/ST/BP_Guard_ST.ST_CurrentDecision` "NewEnumerator1" _asbp_guard_st))))