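; StateTree task for the guard's Search state, moving a BP_Guard_ST actor between search points.
; On state enter, it prints a debug message and, if the guard is idle, requests the next search point and starts moving there.
; Each tick it repeats that request while STWantsSearch is set and the guard is not moving.
; Point selection and movement live in the guard Blueprint, and the task never finishes itself.
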(event `self.ReceiveLatentEnterState`
  (params (Transition :type "StateTreeTransitionResult Structure (by ref)"))
  (bind _asbp_guard_st (cast `/Game/0-Main/Scenarios/Test1/Blueprints/ST/BP_Guard_ST` (`self.Actor`)))
  (`KismetSystemLibrary.PrintString` "\"ST STATE: SEARCH")
  (if (not (`/Game/0-Main/Scenarios/Test1/Blueprints/BP_Guard_Base.bIsMovingToTarget` _asbp_guard_st))
    (bind (_found _location) (`/Game/0-Main/Scenarios/Test1/Blueprints/BP_Guard_Base.GetNextSearchPoint` _asbp_guard_st))
    (if _found
      (`/Game/0-Main/Scenarios/Test1/Blueprints/BP_Guard_Base.StartMoveToSearchPoint` _asbp_guard_st _location))))

(event `self.ReceiveLatentTick`
  (params (DeltaTime :type "Float (single-precision)"))
  (bind _asbp_guard_st (cast `/Game/0-Main/Scenarios/Test1/Blueprints/ST/BP_Guard_ST` (`self.Actor`)))
  (if (`/Game/0-Main/Scenarios/Test1/Blueprints/ST/BP_Guard_ST.ST_WantsSearch` _asbp_guard_st)
    (if (not (`/Game/0-Main/Scenarios/Test1/Blueprints/BP_Guard_Base.bIsMovingToTarget` _asbp_guard_st))
      (bind (_found _location) (`/Game/0-Main/Scenarios/Test1/Blueprints/BP_Guard_Base.GetNextSearchPoint` _asbp_guard_st))
      (if _found
        (`/Game/0-Main/Scenarios/Test1/Blueprints/BP_Guard_Base.StartMoveToSearchPoint` _asbp_guard_st _location)))))