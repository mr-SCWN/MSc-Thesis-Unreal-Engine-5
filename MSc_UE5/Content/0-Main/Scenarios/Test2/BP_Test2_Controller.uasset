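; Scenario controller for Test2, which sets up a seeded item catalog and seller dialog test when StartScenario receives a config.
; It copies the Test2 settings, seeds a random stream, then fills CatalogRows with unique, randomly drawn ItemsDT row names, without using CatalogSize as a limit.
; It prints the setup and shows a dialog widget summarizing the settings.
; GetScenarioName returns an empty string.
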(event `/Game/0-Main/Core/Interfaces/BPI_TestScenario.StartScenario`
  (params (TestConfig :type "/Game/0-Main/Core/Configs/DA_TestConfig Object Reference"))
  (bind (_global_runid _global_enablecsvprofiler _global_timelimittmax _global_seed) (break `/Game/0-Main/Core/Structs/S_GlobalSettings` (`/Game/0-Main/Core/Configs/DA_TestConfig.Global` (`self.ConfigRef`))))
  (bind (_test2_catalogsize _test2_criteriacount _test2_dialogoptionscount _test2_sellergoalmode _test2_playerprofile) (break `/Game/0-Main/Core/Structs/S_Test2Settings` (`/Game/0-Main/Core/Configs/DA_TestConfig.Test2` (`self.ConfigRef`))))
  (set `self.ConfigRef` TestConfig)
  (`KismetMathLibrary.SetRandomStreamSeed` (`self.RandomStream`) _global_seed)
  (set `self.CatalogSize` _test2_catalogsize)
  (set `self.CriteraCount` _test2_criteriacount)
  (set `self.DialogOptionCount` _test2_dialogoptionscount)
  (set `self.SellerGoalMode` _test2_sellergoalmode)
  (set `self.PlayerProfile` _test2_playerprofile)
  (bind _outrownames (`DataTableFunctionLibrary.GetDataTableRowNames` (`self.ItemsDT`)))
  (`KismetArrayLibrary.Array_Clear` (`self.CatalogRows`))
  (bind _returnvalue (- (`KismetArrayLibrary.Array_Length` _outrownames) 1))
  (for _ (range (+ (* _returnvalue 5) 1))
    (`KismetArrayLibrary.Array_AddUnique` (`self.CatalogRows`) (`|GetArrayItem` _outrownames (`KismetMathLibrary.RandomIntegerFromStream` (`self.RandomStream`) _returnvalue))))
  (`KismetSystemLibrary.PrintString` (`KismetStringLibrary.Concat_StrStr` "TEST2 START" (`KismetStringLibrary.Concat_StrStr` "CatalogSize=" (`KismetStringLibrary.Conv_IntToString` (`self.CatalogSize`)) ";") (`KismetStringLibrary.Concat_StrStr` "CatalogRows.length=" (`KismetStringLibrary.Conv_IntToString` (`KismetArrayLibrary.Array_Length` (`self.CatalogRows`))) ";") (`KismetStringLibrary.Concat_StrStr` "CriteriaCount=" (`KismetStringLibrary.Conv_IntToString` (`self.CriteraCount`)) ";") (`KismetStringLibrary.Concat_StrStr` "DialogOptionsCount=" (`KismetStringLibrary.Conv_IntToString` (`self.DialogOptionCount`)) ";") (`KismetStringLibrary.Concat_StrStr` "SellerGoal=" (`KismetStringLibrary.Conv_ByteToString` (`self.SellerGoalMode`)) ";") (`KismetStringLibrary.Concat_StrStr` "PlayerProfile=" (`KismetStringLibrary.Conv_ByteToString` (`self.PlayerProfile`)) ";")))
  (bind _returnvalue_2 (`|CreateWidget` (`self.DialogWidgetClass`) (`GameplayStatics.GetPlayerController` 0) (`|FormatText` "Catalog={Catalog} | Criteria={Criteria} | Dialog={Dialog} | Goal={Goal} | Profile={Profile}" (`self.CatalogSize`) (`self.CriteraCount`) (`self.DialogOptionCount`) (`self.SellerGoalMode`) (`self.PlayerProfile`))))
  (`UserWidget.AddToViewport` _returnvalue_2 0)
  (set `self.DialogWidgetInstance` _returnvalue_2))

(fn `GetScenarioName`
  (returns (GetScenarioName :type String))
  (return ""))

(fn `UserConstructionScript`)