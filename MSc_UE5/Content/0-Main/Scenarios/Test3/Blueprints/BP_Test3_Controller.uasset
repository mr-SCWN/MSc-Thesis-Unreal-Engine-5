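; Controller for the Test3 scenario, which configures shelters and spawns NPCs from a test config when StartScenario runs.
; Map change mode selects the closed-shelter list that drives each shelter's open state, while capacity mode sets zero, equal or alternating ±50% capacity from the NPC count.
; It then clears earlier NPCs and spawns new ones within SpawnArea using a seeded random stream.
; RegisterSavedNPC and GetScenarioName are empty stubs.
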(event `/Game/0-Main/Core/Interfaces/BPI_TestScenario.StartScenario`
  (params (TestConfig :type "/Game/0-Main/Core/Configs/DA_TestConfig Object Reference"))
  (bind _spawnednpcs (`self.SpawnedNPCs`))
  (bind _spawnarea (`self.SpawnArea`))
  (bind (_test3_npccountm _test3_sheltercapacitymode _test3_mapchangemode _test3_closedshelters_20 _test3_closedshelters_50) (break `/Game/0-Main/Core/Structs/S_Test3Settings` (`/Game/0-Main/Core/Configs/DA_TestConfig.Test3` (`self.ConfigRef`))))
  (bind _x (.x (`BoxComponent.GetScaledBoxExtent` _spawnarea)))
  (bind _y (.y (`BoxComponent.GetScaledBoxExtent` _spawnarea)))
  (bind _returnvalue (`KismetMathLibrary.FCeil` (/ (`self.NPCCountM`) (- 10 (`KismetArrayLibrary.Array_Length` (`self.ClosedList`))))))
  (bind _returnvalue_2 (`KismetMathLibrary.FCeil` (* _returnvalue 0.5)))
  (bind _output_get (set `self.ConfigRef` TestConfig))
  (bind (_global_runid _global_enablecsvprofiler _global_timelimittmax _global_seed) (break `/Game/0-Main/Core/Structs/S_GlobalSettings` (`/Game/0-Main/Core/Configs/DA_TestConfig.Global` _output_get)))
  (`KismetMathLibrary.SetRandomStreamSeed` (`self.RandomStream`) _global_seed)
  (set `self.NPCCountM` _test3_npccountm)
  (set `self.ShelterCapacityMode` _test3_sheltercapacitymode)
  (set `self.MapChangeMode` _test3_mapchangemode)
  (set `self.ClosedShelters_20` _test3_closedshelters_20)
  (set `self.ClosedShelters_50` _test3_closedshelters_50)
  (bind _outactors (`GameplayStatics.GetAllActorsOfClass` "/Game/0-Main/Scenarios/Test3/Blueprints/BP_Shelter.BP_Shelter_C"))
  (for (_array_element _array_index) _outactors
    (`KismetArrayLibrary.Array_Add` (`self.AllShelters`) _array_element)
    (set `/Game/0-Main/Scenarios/Test3/Blueprints/BP_Shelter.Occupacy` 0 _array_element)
    (`/Game/0-Main/Scenarios/Test3/Blueprints/BP_Shelter.SetOpen` _array_element false)
    (if (== (`self.MapChangeMode`) 0)
      (if (`KismetArrayLibrary.Array_Contains` (`self.ClosedList`) (`/Game/0-Main/Scenarios/Test3/Blueprints/BP_Shelter.ShelterID` _array_element)) :!label _label
        (`/Game/0-Main/Scenarios/Test3/Blueprints/BP_Shelter.SetOpen` _array_element true)
        (if (== (`self.ShelterCapacityMode`) 0)
          (set `/Game/0-Main/Scenarios/Test3/Blueprints/BP_Shelter.Capacity` 0 _array_element)
          (elif (== (`self.ShelterCapacityMode`) 1)
            (set `/Game/0-Main/Scenarios/Test3/Blueprints/BP_Shelter.Capacity` _returnvalue _array_element)
            (elif (== (`self.ShelterCapacityMode`) 2)
              (if (== (mod _array_index 2) 0)
                (set `/Game/0-Main/Scenarios/Test3/Blueprints/BP_Shelter.Capacity` (+ _returnvalue _returnvalue_2) _array_element)
                (else
                  (set `/Game/0-Main/Scenarios/Test3/Blueprints/BP_Shelter.Capacity` (- _returnvalue _returnvalue_2) _array_element)))))))
      (elif (== (`self.MapChangeMode`) 1)
        (set `self.ClosedList` (`self.ClosedShelters_20`))
        (goto _label)
        (elif (== (`self.MapChangeMode`) 2)
          (set `self.ClosedList` (`self.ClosedShelters_50`))
          (goto _label)))))
  (for _array_element_2 _spawnednpcs
    (`self.K2_DestroyActor` _array_element_2)
    (`KismetArrayLibrary.Array_Clear` _spawnednpcs))
  (for _ (range (`self.NPCCountM`))
    (bind _returnvalue_3 (`|SpawnActorFromClass` (`self.NPCClass`) (`KismetMathLibrary.MakeTransform` (+ (`SceneComponent.K2_GetComponentLocation` _spawnarea) (`KismetMathLibrary.MakeVector` (`KismetMathLibrary.RandomFloatInRangeFromStream` (`self.RandomStream`) (* _x -1.0) _x) (`KismetMathLibrary.RandomFloatInRangeFromStream` (`self.RandomStream`) (* _y -1.0) _y)))) "Undefined" "MultiplyWithRoot" null null))
    (`KismetArrayLibrary.Array_Add` (`self.SpawnedNPCs`) _returnvalue_3)))

(fn `GetScenarioName`
  (returns (GetScenarioName :type String))
  (return ""))

(fn `RegisterSavedNPC`
  (params (NPC :type "/Game/0-Main/Scenarios/Test3/Blueprints/BP_NPCDummy Object Reference") (Shelter :type "/Game/0-Main/Scenarios/Test3/Blueprints/BP_Shelter Object Reference")))

(fn `UserConstructionScript`)