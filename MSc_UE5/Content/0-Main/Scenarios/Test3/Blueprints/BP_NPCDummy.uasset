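; Evacuee NPC for the Test3 shelter scenario, initialized by a controller as Cooperative or Egoist and colored by role.
; A looping think timer picks the nearest shelter not known closed or full, then AI-moves there to attempt entry.
; Refusals are remembered and trigger retries; success hides the NPC and notifies the controller.
; Cooperative NPCs share bad-shelter knowledge within ComRadius (not the initialized CommunicationRadius), making receivers retarget and tracking counters.
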(event `self.ReceiveBeginPlay`
  (`self.ApplyRoleVisual`))

(event `EvacThink`
  (if (`self.bSaved `)
    _
    (elif (`self.bEvacuating `)
      (`self.ShareInformationIfCooperative`)
      (if (not (`self.bMovingToShelter `))
        (bind _selectedshelter_ (`self.DecideNextShelter`))
        (if (`KismetSystemLibrary.IsValid` _selectedshelter_)
          (`self.StartMoveToShelter` _selectedshelter_)
          (else
            (`KismetSystemLibrary.PrintString` "NPC NO SHELTER AVAILABLE")))))))

(event `StartMoveToShelter`
  (params (Shelter :type "/Game/0-Main/Scenarios/Test3/Blueprints/BP_Shelter Object Reference"))
  (bind _currentshelter_ (`self.CurrentShelter `))
  (bind _currentshelter__2 (`self.CurrentShelter `))
  (if (`KismetSystemLibrary.IsValid` Shelter)
    (if (and (!= _currentshelter_ Shelter) (`KismetSystemLibrary.IsValid` _currentshelter_))
      (set `self.TargetChangeCount ` (+ (`self.TargetChangeCount `) 1)))
    (bind _output_get (set `self.CurrentShelter ` Shelter))
    (set `self.bMovingToShelter ` true)
    (bind (_projectedlocation _returnvalue) (`NavigationSystemV1.K2_ProjectPointToNavigation` (`self.K2_GetActorLocation` _output_get) null null (500.0 500.0 500.0)))
    (if _returnvalue
      (`|AIMoveTo` self _projectedlocation Shelter 150.0
        (:`OnSuccess`
          (set `self.bMovingToShelter ` false)
          (if (`self.bSaved `)
            _
            (elif (`KismetSystemLibrary.IsValid` _currentshelter__2)
              (bind _shelterenterresult (`/Game/0-Main/Scenarios/Test3/Blueprints/BP_Shelter.TryEnterShelter` _currentshelter__2 self))
              (`self.HandleShelterResult` _currentshelter__2 _shelterenterresult))))
        (:`OnFail`
          (set `self.bMovingToShelter ` false)
          (set `self.CurrentShelter ` null)
          (`KismetSystemLibrary.PrintString` "MOVE TO SHELTER FAILED")))
      (else
        (set `self.bMovingToShelter ` false)
        (set `self.CurrentShelter ` null)
        (`KismetSystemLibrary.PrintString` "SHELTER LOCATION NOT ON NAVMESH")))
    (else
      (`KismetSystemLibrary.PrintString` "START MOVE: INVALID SHELTER"))))

(fn `ApplyRoleVisual`
  (if (== (`self.Rolee`) 0)
    (`PrimitiveComponent.SetMaterial` (`self.BodyMesh`) 0 "/Game/0-Main/Scenarios/Test3/Materials/M_MatGood.M_MatGood")
    (elif (== (`self.Rolee`) 1)
      (`PrimitiveComponent.SetMaterial` (`self.BodyMesh`) 0 "/Game/0-Main/Scenarios/Test3/Materials/M_MatEgoist.M_MatEgoist")
      (elif (== (`self.Rolee`) 2)
        (`PrimitiveComponent.SetMaterial` (`self.BodyMesh`) 0 "/Game/0-Main/Scenarios/Test3/Materials/M_MatScout.M_MatScout")))))

(fn `DecideNextShelter`
  (returns (`SelectedShelter ` :type "/Game/0-Main/Scenarios/Test3/Blueprints/BP_Shelter Object Reference"))
  (locals (`BestShelter ` :type "/Game/0-Main/Scenarios/Test3/Blueprints/BP_Shelter Object Reference") (`BestDistance ` :type "Float (double-precision)") (`CurrentDistance ` :type "Float (double-precision)"))
  (set `local.BestShelter ` null)
  (set `local.BestDistance ` 99999999.0)
  (for _array_element (`self.AllShelters`)
    (if (`KismetSystemLibrary.IsValid` _array_element)
      (if (not (or (`KismetArrayLibrary.Array_Contains` (`self.KnownClosedShelters `) _array_element) (`KismetArrayLibrary.Array_Contains` (`self.KnownFullShelters `) _array_element)))
        (set `local.CurrentDistance ` (`KismetMathLibrary.Vector_Distance` (`self.K2_GetActorLocation` _array_element) (`self.K2_GetActorLocation`)))
        (if (< (`local.CurrentDistance `) (`local.BestDistance `))
          (set `local.BestDistance ` (`local.CurrentDistance `))
          (set `local.BestShelter ` _array_element)))))
  (return (`local.BestShelter `)))

(fn `HandleShelterResult`
  (params (Shelter :type "/Game/0-Main/Scenarios/Test3/Blueprints/BP_Shelter Object Reference") (`Result ` :type "/Game/0-Main/Scenarios/Test3/Blueprints/E_ShelterEnterResult Enum" :default "NewEnumerator0"))
  (bind _test3controller_ (`self.Test3Controller `))
  (if (not (`self.bSaved `))
    (switch `/Game/0-Main/Scenarios/Test3/Blueprints/E_ShelterEnterResult` `Result `
      (:`NewEnumerator0`
        (set `self.bSaved ` true)
        (set `self.bEvacuating ` false)
        (set `self.bMovingToShelter ` false)
        (`KismetSystemLibrary.K2_ClearAndInvalidateTimerHandle` (`self.EvacThinkTimerHandle `))
        (`KismetSystemLibrary.PrintString` "NPC SAVED")
        (if (`KismetSystemLibrary.IsValid` _test3controller_)
          (`/Game/0-Main/Scenarios/Test3/Blueprints/BP_Test3_Controller.RegisterSavedNPC` _test3controller_ self Shelter))
        (`CharacterMovementComponent.DisableMovement` (`self.CharacterMovement`))
        (`self.SetActorEnableCollision` false)
        (`self.SetActorHiddenInGame` true))
      (:`NewEnumerator1`
        (`KismetArrayLibrary.Array_AddUnique` (`self.KnownClosedShelters `) Shelter)
        (set `self.FailedShelterAttempts ` (+ (`self.FailedShelterAttempts `) 1))
        (set `self.CurrentShelter ` null)
        (set `self.bMovingToShelter ` false)
        (`KismetSystemLibrary.PrintString` "SHELTER CLOSED")
        (`self.ShareInformationIfCooperative`)
        (`self.EvacThink`))
      (:`NewEnumerator2`
        (`KismetArrayLibrary.Array_AddUnique` (`self.KnownFullShelters `) Shelter)
        (set `self.FailedShelterAttempts ` (+ (`self.FailedShelterAttempts `) 1))
        (set `self.CurrentShelter ` null)
        (set `self.bMovingToShelter ` false)
        (`KismetSystemLibrary.PrintString` "SHELTER FULL")
        (`self.ShareInformationIfCooperative`)
        (`self.EvacThink`)))))

(fn `InitEvacNPC`
  (params (`SheltersIn ` :type "Array of /Game/0-Main/Scenarios/Test3/Blueprints/BP_Shelter Object Reference") (`ControllerIn ` :type "/Game/0-Main/Scenarios/Test3/Blueprints/BP_Test3_Controller Object Reference") (`NPCTypeIn ` :type "/Game/0-Main/Scenarios/Test3/Blueprints/E_EvacNPCType Enum" :default "NewEnumerator0") (`CommunicationRadiusIn ` :type "Float (double-precision)"))
  (set `self.AllShelters` `SheltersIn `)
  (set `self.Test3Controller ` `ControllerIn `)
  (set `self.NPCType ` `NPCTypeIn `)
  (set `self.CommunicationRadius ` `CommunicationRadiusIn `)
  (`KismetArrayLibrary.Array_Clear` (`self.KnownClosedShelters `))
  (`KismetArrayLibrary.Array_Clear` (`self.KnownFullShelters `))
  (set `self.CurrentShelter ` null)
  (set `self.bEvacuating ` false)
  (set `self.bSaved ` false)
  (set `self.bMovingToShelter ` false)
  (set `self.TargetChangeCount ` 0)
  (set `self.FailedShelterAttempts ` 0)
  (set `self.InfoReceivedCount ` 0)
  (switch `/Game/0-Main/Scenarios/Test3/Blueprints/E_EvacNPCType` (`self.NPCType `)
    (:`NewEnumerator0`
      (set `self.Rolee` 0))
    (:`NewEnumerator1`
      (set `self.Rolee` 1)))
  (`self.ApplyRoleVisual`))

(fn `IsShelterKnownBad`
  (params (Shelter :type "/Game/0-Main/Scenarios/Test3/Blueprints/BP_Shelter Object Reference"))
  (returns (IsBad :type Boolean))
  (if (or (`KismetArrayLibrary.Array_Contains` (`self.KnownFullShelters `) Shelter) (`KismetArrayLibrary.Array_Contains` (`self.KnownClosedShelters `) Shelter))
    (return true)
    (else
      (return false))))

(fn `ReceiveShelterInfo`
  (params (`ClosedIn ` :type "Array of /Game/0-Main/Scenarios/Test3/Blueprints/BP_Shelter Object Reference") (FullIn :type "Array of /Game/0-Main/Scenarios/Test3/Blueprints/BP_Shelter Object Reference"))
  (locals (NewInfo :type Boolean) (`CurrentTargetBecameBad ` :type Boolean))
  (bind _returnvalue (`self.GetController`))
  (set `local.NewInfo` false)
  (set `local.CurrentTargetBecameBad ` false)
  (for _array_element `ClosedIn `
    (if (`KismetSystemLibrary.IsValid` _array_element)
      (if (not (`KismetArrayLibrary.Array_Contains` (`self.KnownClosedShelters `) _array_element))
        (`KismetArrayLibrary.Array_AddUnique` (`self.KnownClosedShelters `) _array_element)
        (set `local.NewInfo` true)
        (if (== _array_element (`self.CurrentShelter `))
          (set `local.CurrentTargetBecameBad ` true)))))
  (for _array_element_2 FullIn
    (if (`KismetSystemLibrary.IsValid` _array_element_2)
      (if (not (`KismetArrayLibrary.Array_Contains` (`self.KnownFullShelters `) _array_element_2))
        (`KismetArrayLibrary.Array_AddUnique` (`self.KnownFullShelters `) _array_element_2)
        (set `local.NewInfo` true)
        (if (== _array_element_2 (`self.CurrentShelter `))
          (set `local.CurrentTargetBecameBad ` true)))))
  (if (`local.NewInfo`)
    (`KismetSystemLibrary.PrintString` "INFO RECEIVED")
    (set `self.InfoReceivedCount ` (+ (`self.InfoReceivedCount `) 1))
    (if (`local.CurrentTargetBecameBad `)
      (if (and (`self.bMovingToShelter `) (not (`self.bSaved `)) (`self.bEvacuating `))
        (if (`KismetSystemLibrary.IsValid` _returnvalue)
          (`Controller.StopMovement` _returnvalue))
        (set `self.bMovingToShelter ` false)
        (set `self.CurrentShelter ` null)
        (set `self.TargetChangeCount ` (+ (`self.TargetChangeCount `) 1))
        (`KismetSystemLibrary.PrintString` "TARGET CHANGED BY INFO")
        (`self.EvacThink`)))))

(fn `ShareInformationIfCooperative`
  (locals (ComRadius :type "Float (double-precision)" :default 900.0))
  (bind _test3controller_ (`self.Test3Controller `))
  (switch `/Game/0-Main/Scenarios/Test3/Blueprints/E_EvacNPCType` (`self.NPCType `)
    (:`NewEnumerator0`
      (if (> (+ (`KismetArrayLibrary.Array_Length` (`self.KnownClosedShelters `)) (`KismetArrayLibrary.Array_Length` (`self.KnownFullShelters `))) 0)
        (if (`KismetSystemLibrary.IsValid` _test3controller_)
          (for _array_element (`/Game/0-Main/Scenarios/Test3/Blueprints/BP_Test3_Controller.SpawnedNPCs` _test3controller_)
            (if (`KismetSystemLibrary.IsValid` _array_element)
              (if (!= _array_element self)
                (if (`/Game/0-Main/Scenarios/Test3/Blueprints/BP_NPCDummy.bSaved ` _array_element)
                  _
                  (elif (<= (`KismetMathLibrary.Vector_Distance` (`self.K2_GetActorLocation`) (`self.K2_GetActorLocation` _array_element)) (`local.ComRadius`))
                    (`self.ReceiveShelterInfo` _array_element (`self.KnownClosedShelters `) (`self.KnownFullShelters `))))))))))))

(fn `StartEvacAI`
  (set `self.bEvacuating ` true)
  (`KismetSystemLibrary.PrintString` "NPC EVAC START")
  (bind _returnvalue (`KismetSystemLibrary.K2_SetTimerDelegate` (`|CreateDelegate` :!event `EvacThink`) (`self.DecisionInterval `) true))
  (set `self.EvacThinkTimerHandle ` _returnvalue)
  (`self.EvacThink`))

(fn `UserConstructionScript`
  (`self.ApplyRoleVisual`))