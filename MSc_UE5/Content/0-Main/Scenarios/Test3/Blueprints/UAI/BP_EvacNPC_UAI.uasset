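; Evacuation NPC variant that overrides shelter choice with utility-style scoring to pick where it goes next.
; DecideNextShelter scores each shelter not known bad using a base score plus a two-tier, range-based distance score.
; It subtracts a crowd penalty, the count of other unsaved NPCs from Test3Controller moving to that shelter times UAIMaxDistance.
; The top-scoring shelter is printed and returned, without calling the parent's decision logic.
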(fn `DecideNextShelter`
  (returns (`SelectedShelter ` :type "/Game/0-Main/Scenarios/Test3/Blueprints/BP_Shelter Object Reference"))
  (locals (`BestShelter ` :type "/Game/0-Main/Scenarios/Test3/Blueprints/BP_Shelter Object Reference") (`BestScore ` :type "Float (double-precision)") (`CandidateScore ` :type "Float (double-precision)") (`CurrentDistance ` :type "Float (double-precision)") (`DistanceScore ` :type "Float (double-precision)") (`CrowdCount ` :type "Float (double-precision)") (`CrowdPenalty ` :type "Float (double-precision)"))
  (set `local.BestShelter ` null)
  (set `local.BestScore ` -999999.0)
  (for _array_element (`self.AllShelters`)
    (if (`KismetSystemLibrary.IsValid` _array_element)
      (bind _isbad (`self.IsShelterKnownBad` _array_element))
      (if (not _isbad)
        (bind _output_get (set `local.CurrentDistance ` (`KismetMathLibrary.Vector_Distance` (`self.K2_GetActorLocation` _array_element) (`self.K2_GetActorLocation`))))
        (bind _score_ (`self.UAI_CalculateDistanceScore` _output_get))
        (set `local.DistanceScore ` _score_)
        (bind _count_ (`self.UAI_CountAgentsTargetingShelter` _array_element))
        (bind _output_get_2 (set `local.CrowdCount ` (`KismetMathLibrary.Conv_IntToDouble` _count_)))
        (set `local.CrowdPenalty ` (* _output_get_2 (`self.UAI_MaxDistance `)))
        (bind _output_get_3 (set `local.CandidateScore ` (- (+ (`self.UAI_BaseScore `) (`local.DistanceScore `)) (`local.CrowdPenalty `))))
        (if (> _output_get_3 (`local.BestScore `))
          (set `local.BestScore ` (`local.CandidateScore `))
          (set `local.BestShelter ` _array_element)))))
  (`KismetSystemLibrary.PrintString` (`KismetStringLibrary.Concat_StrStr` "UAI bot  " (`KismetStringLibrary.Conv_ObjectToString` self) "SELECTED SHELTER" (`KismetStringLibrary.Conv_ObjectToString` (`local.BestShelter `))))
  (return (`local.BestShelter `)))

(fn `UAI_CalculateDistanceScore`
  (params (`Distance ` :type "Float (double-precision)"))
  (returns (`Score ` :type "Float (double-precision)"))
  (if (`KismetMathLibrary.InRange_FloatFloat` `Distance ` 0.0 (`self.UAI_MaxDistance `))
    (return (`self.UAI_BaseScore `))
    (else
      (return 100.0))))

(fn `UAI_CountAgentsTargetingShelter`
  (params (Shelter :type "/Game/0-Main/Scenarios/Test3/Blueprints/BP_Shelter Object Reference"))
  (returns (`Count ` :type Integer))
  (locals (localCount :type Integer))
  (bind _test3controller_ (`self.Test3Controller `))
  (set `local.localCount` 0)
  (if (`KismetSystemLibrary.IsValid` _test3controller_)
    (for _array_element (`/Game/0-Main/Scenarios/Test3/Blueprints/BP_Test3_Controller.SpawnedNPCs` _test3controller_)
      (if (`KismetSystemLibrary.IsValid` _array_element)
        (if (!= _array_element self)
          (if (`/Game/0-Main/Scenarios/Test3/Blueprints/BP_NPCDummy.bSaved ` _array_element)
            _
            (elif (`/Game/0-Main/Scenarios/Test3/Blueprints/BP_NPCDummy.bMovingToShelter ` _array_element)
              (if (== (`/Game/0-Main/Scenarios/Test3/Blueprints/BP_NPCDummy.CurrentShelter ` _array_element) Shelter)
                (set `local.localCount` (+ (`local.localCount`) 1))))))))
    (return (`local.localCount`))
    (else
      (return 0))))

(fn `UserConstructionScript`
  (`parent.UserConstructionScript`))