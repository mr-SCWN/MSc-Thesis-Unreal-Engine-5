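; BP_Shelter is a shelter actor that dummy NPCs try to enter, with an ID label and an open or closed material.
; Overlapping its trigger admits only unsaved NPCs moving to this shelter, provided it is open and has space, with optional unlimited capacity.
; It increments occupancy on entry and passes an entered, closed or full result back to the NPC to handle.
; SetOpen and the construction script both refresh the visual state.
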(event `self.EnterTrigger.OnComponentBeginOverlap`
  (params (OverlappedComponent :type "PrimitiveComponent Object Reference") (OtherActor :type "Actor Object Reference") (OtherComp :type "PrimitiveComponent Object Reference") (OtherBodyIndex :type Integer) (bFromSweep :type Boolean) (SweepResult :type "HitResult Structure (by ref)"))
  (bind _asbp_npcdummy (cast `/Game/0-Main/Scenarios/Test3/Blueprints/BP_NPCDummy` OtherActor))
  (if (and (== (`/Game/0-Main/Scenarios/Test3/Blueprints/BP_NPCDummy.bMovingToShelter ` _asbp_npcdummy) true) (== (`/Game/0-Main/Scenarios/Test3/Blueprints/BP_NPCDummy.bSaved ` _asbp_npcdummy) false) (== (`/Game/0-Main/Scenarios/Test3/Blueprints/BP_NPCDummy.CurrentShelter ` _asbp_npcdummy) self))
    (bind _shelterenterresult (`self.TryEnterShelter` _asbp_npcdummy))
    (`/Game/0-Main/Scenarios/Test3/Blueprints/BP_NPCDummy.HandleShelterResult` _asbp_npcdummy self _shelterenterresult)))

(fn `ApplyVisualState`
  (`TextRenderComponent.K2_SetText` (`self.IDText`) (`|GenericToText` (`self.ShelterID`)))
  (if (`self.bIsOpen`)
    (`PrimitiveComponent.SetMaterial` (`self.ShelterMesh`) 0 (`self.Mat_Open`))
    (else
      (`PrimitiveComponent.SetMaterial` (`self.ShelterMesh`) 0 (`self.Mat_Closed`)))))

(fn `HasFreePlace`
  (returns (FreePlace :type Boolean))
  (if (`self.bUnlimitedCapacity `)
    (return true)
    (else
      (return (> (`self.Capacity`) (`self.Occupacy`))))))

(fn `SetOpen`
  (params (NewOpen :type Boolean))
  (set `self.bIsOpen` NewOpen)
  (`self.ApplyVisualState`))

(fn `TryEnterShelter`
  (params (NPC :type "/Game/0-Main/Scenarios/Test3/Blueprints/BP_NPCDummy Object Reference"))
  (returns (ShelterEnterResult :type "/Game/0-Main/Scenarios/Test3/Blueprints/E_ShelterEnterResult Enum"))
  (if (`self.bIsOpen`)
    (bind _freeplace (`self.HasFreePlace`))
    (if _freeplace
      (set `self.Occupacy` (+ (`self.Occupacy`) 1))
      (return "NewEnumerator0")
      (else
        (return "NewEnumerator2")))
    (else
      (return "NewEnumerator1"))))

(fn `UserConstructionScript`
  (`self.ApplyVisualState`))