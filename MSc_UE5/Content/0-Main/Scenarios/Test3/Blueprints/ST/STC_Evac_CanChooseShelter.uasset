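; StateTree condition for the Test3 evacuation scenario that decides whether an evacuee pawn can choose a shelter.
; It passes only when the EvacPawn is valid, is evacuating, and is neither already moving to a shelter nor saved.
; An invalid pawn fails the condition.
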(fn `ReceiveTestCondition`
  (returns (ReturnValue :type Boolean))
  (bind _evacpawn (`self.EvacPawn`))
  (if (`KismetSystemLibrary.IsValid` _evacpawn)
    (return (and (not (`/Game/0-Main/Scenarios/Test3/Blueprints/BP_NPCDummy.bMovingToShelter ` _evacpawn)) (not (`/Game/0-Main/Scenarios/Test3/Blueprints/BP_NPCDummy.bSaved ` _evacpawn)) (`/Game/0-Main/Scenarios/Test3/Blueprints/BP_NPCDummy.bEvacuating ` _evacpawn)))
    (else
      (return false))))