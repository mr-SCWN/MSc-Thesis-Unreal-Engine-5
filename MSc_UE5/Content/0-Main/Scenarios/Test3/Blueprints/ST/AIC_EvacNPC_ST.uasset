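; AI controller for evacuation NPCs (BP_NPCDummy) that runs a State Tree deciding when they share information and move to shelters.
; StartEvacST starts the StateTreeAI component's logic, with debug prints.
; ST_-prefixed functions wrap the pawn's Saved, Evacuating and MovingToShelter flags as state checks.
; Action wrappers trigger cooperative information sharing, or pick the next shelter and start movement, returning success or failure.
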(fn `GetEvacPawn`
  (returns (`EvacPawn ` :type "/Game/0-Main/Scenarios/Test3/Blueprints/BP_NPCDummy Object Reference"))
  (bind _asbp_npcdummy (cast `/Game/0-Main/Scenarios/Test3/Blueprints/BP_NPCDummy` (`self.K2_GetPawn`))
    (:`then`
      (return _asbp_npcdummy))
    (:`CastFailed`
      (return null))))

(fn `ST_CanChooseShelter`
  (returns (Result :type Boolean))
  (bind _evacpawn_ (`self.GetEvacPawn`))
  (if (`KismetSystemLibrary.IsValid` _evacpawn_)
    (return (and (not (`/Game/0-Main/Scenarios/Test3/Blueprints/BP_NPCDummy.bSaved ` _evacpawn_)) (`/Game/0-Main/Scenarios/Test3/Blueprints/BP_NPCDummy.bEvacuating ` _evacpawn_) (not (`/Game/0-Main/Scenarios/Test3/Blueprints/BP_NPCDummy.bMovingToShelter ` _evacpawn_))))
    (else
      (return false))))

(fn `ST_IsMoving`
  (returns (REsult :type Boolean))
  (bind _evacpawn_ (`self.GetEvacPawn`))
  (if (`KismetSystemLibrary.IsValid` _evacpawn_)
    (return (and (`/Game/0-Main/Scenarios/Test3/Blueprints/BP_NPCDummy.bMovingToShelter ` _evacpawn_) (not (`/Game/0-Main/Scenarios/Test3/Blueprints/BP_NPCDummy.bSaved ` _evacpawn_))))
    (else
      (return false))))

(fn `ST_IsSaved`
  (returns (Result :type Boolean))
  (bind _evacpawn_ (`self.GetEvacPawn`))
  (if (`KismetSystemLibrary.IsValid` _evacpawn_)
    (return (`/Game/0-Main/Scenarios/Test3/Blueprints/BP_NPCDummy.bSaved ` _evacpawn_))
    (else
      (return false))))

(fn `ST_SelectAndStartMove`
  (returns (Resuilt :type Boolean))
  (bind _evacpawn_ (`self.GetEvacPawn`))
  (if (`KismetSystemLibrary.IsValid` _evacpawn_)
    (if (and (not (`/Game/0-Main/Scenarios/Test3/Blueprints/BP_NPCDummy.bSaved ` _evacpawn_)) (`/Game/0-Main/Scenarios/Test3/Blueprints/BP_NPCDummy.bEvacuating ` _evacpawn_) (not (`/Game/0-Main/Scenarios/Test3/Blueprints/BP_NPCDummy.bMovingToShelter ` _evacpawn_)))
      (bind _selectedshelter_ (`/Game/0-Main/Scenarios/Test3/Blueprints/BP_NPCDummy.DecideNextShelter` _evacpawn_))
      (if (`KismetSystemLibrary.IsValid` _selectedshelter_)
        (`/Game/0-Main/Scenarios/Test3/Blueprints/BP_NPCDummy.StartMoveToShelter` _evacpawn_ _selectedshelter_)
        (`KismetSystemLibrary.PrintString` "ST START MOVE")
        (return true)
        (else
          (`KismetSystemLibrary.PrintString` "ST NO SHELTER")
          (return false)))
      (else
        (return false)))
    (else
      (return false))))

(fn `ST_UpdateCommunication`
  (returns (Result :type Boolean))
  (bind _evacpawn_ (`self.GetEvacPawn`))
  (if (`KismetSystemLibrary.IsValid` _evacpawn_)
    (`/Game/0-Main/Scenarios/Test3/Blueprints/BP_NPCDummy.ShareInformationIfCooperative` _evacpawn_)
    (return true)
    (else
      (return false))))

(fn `StartEvacST`
  (bind _statetreeai (`self.StateTreeAI`))
  (if (`KismetSystemLibrary.IsValid` _statetreeai)
    (`BrainComponent.StartLogic` _statetreeai)
    (`KismetSystemLibrary.PrintString` "ST RUN")
    (else
      (`KismetSystemLibrary.PrintString` "ST COMPONENT INVALID"))))

(fn `UserConstructionScript`)