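; BP_EvacNPC_ST is the ST variant of an evacuation NPC in the Test3 scenario.
; Its StartEvacAI override sets Evacuating, clears Saved and MovingToShelter, then calls StartEvacST on its AIC_EvacNPC_ST controller.
; The parent StartEvacAI is never called, so this logic replaces it, with debug prints for start and failed controller cast.
; The event graph holds only disabled stubs.
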(fn `StartEvacAI`
  (set `self.bEvacuating ` true)
  (set `self.bSaved ` false)
  (set `self.bMovingToShelter ` false)
  (`KismetSystemLibrary.PrintString` "ST EVAC START")
  (bind _asaic_evac_npc_st (cast `/Game/0-Main/Scenarios/Test3/Blueprints/ST/AIC_EvacNPC_ST` (`self.GetController`))
    (:`then`
      (`/Game/0-Main/Scenarios/Test3/Blueprints/ST/AIC_EvacNPC_ST.StartEvacST` _asaic_evac_npc_st))
    (:`CastFailed`
      (`KismetSystemLibrary.PrintString` "ST CONTROLLER INVALID"))))

(fn `UserConstructionScript`
  (`parent.UserConstructionScript`))