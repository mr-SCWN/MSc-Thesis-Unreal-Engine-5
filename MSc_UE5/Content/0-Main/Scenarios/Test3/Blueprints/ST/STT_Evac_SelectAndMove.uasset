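; StateTree task that has an evacuee pawn pick a shelter and start moving to it in an evacuation scenario.
; On entering the state, it acts only if the pawn is evacuating, not already moving and not saved, calling DecideNextShelter and passing the result to StartMoveToShelter.
; The task finishes immediately without awaiting arrival, reporting success even when no shelter is found and failure only for an invalid pawn.
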(event `self.ReceiveLatentEnterState`
  (params (Transition :type "StateTreeTransitionResult Structure (by ref)"))
  (bind _evacpawn (`self.EvacPawn`))
  (if (`KismetSystemLibrary.IsValid` _evacpawn)
    (if (and (not (`/Game/0-Main/Scenarios/Test3/Blueprints/BP_NPCDummy.bMovingToShelter ` _evacpawn)) (not (`/Game/0-Main/Scenarios/Test3/Blueprints/BP_NPCDummy.bSaved ` _evacpawn)) (`/Game/0-Main/Scenarios/Test3/Blueprints/BP_NPCDummy.bEvacuating ` _evacpawn))
      (bind _selectedshelter_ (`/Game/0-Main/Scenarios/Test3/Blueprints/BP_NPCDummy.DecideNextShelter` _evacpawn))
      (if (`KismetSystemLibrary.IsValid` _selectedshelter_)
        (`/Game/0-Main/Scenarios/Test3/Blueprints/BP_NPCDummy.StartMoveToShelter` (`self.EvacPawn`) _selectedshelter_)
        (`KismetSystemLibrary.PrintString` "ST START MOVE")
        (`self.FinishTask` true)
        (else
          (`KismetSystemLibrary.PrintString` "ST NO SHELTER")
          (`self.FinishTask` true)))
      (else
        (`self.FinishTask` true)))
    (else
      (`KismetSystemLibrary.PrintString` "ST PAWN INVALID")
      (`self.FinishTask` false))))