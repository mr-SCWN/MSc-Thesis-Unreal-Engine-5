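; BP_TestManager runs timed performance tests on a level, driving a scenario actor through BPI_TestScenario messages.
; StartRun, optionally automatic at BeginPlay, picks the override or first interface actor, resets stats, starts CSV profiling and sets the time-limit timer from ActiveConfig.
; Tick accumulates FPS and frame-time min, max and sum from DeltaSeconds.
; StopRun ends the scenario and profiling, computes averages and prints a RUN_END summary.
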(event `self.ReceiveBeginPlay`
  (if (`self.bAutoStart`)
    (`self.StartRun`)))

(event `StartRun`
  (bind _scenariocontrolleroverride (`self.ScenarioControllerOverride`))
  (bind (_global_runid _global_enablecsvprofiler _global_timelimittmax) (break `/Game/0-Main/Core/Structs/S_GlobalSettings` (`/Game/0-Main/Core/Configs/DA_TestConfig.Global` (`self.ActiveConfig`))))
  (set `self.bRunActive` true)
  (if (`KismetSystemLibrary.IsValid` (`self.ActiveConfig`))
    (if (`KismetSystemLibrary.IsValid` _scenariocontrolleroverride)
      (set `self.ScenarioActor` _scenariocontrolleroverride)
      (set `self.FPS_Min` 9999.0 :!label _label)
      (set `self.FPS_Max` 0.0)
      (set `self.FPS_Sum` 0.0)
      (set `self.FPS_Count` 0)
      (set `self.Frame_Min` 9999.0)
      (set `self.Frame_Max` 0.0)
      (set `self.Frame_Sum` 0.0)
      (set `self.Frame_Count` 0)
      (`KismetSystemLibrary.ExecuteConsoleCommand` "csvprofile start" null)
      (message `/Game/0-Main/Core/Interfaces/BPI_TestScenario.StartScenario` (`self.ScenarioActor`) (`self.ActiveConfig`))
      (`KismetSystemLibrary.K2_SetTimerDelegate` (delegate `StopRun`) _global_timelimittmax)
      (else
        (bind _outactors (`GameplayStatics.GetAllActorsWithInterface` "/Game/0-Main/Core/Interfaces/BPI_TestScenario.BPI_TestScenario_C"))
        (bind _output (`|GetArrayItem` _outactors))
        (if (`KismetSystemLibrary.IsValid` _output)
          (set `self.ScenarioActor` _output)
          (goto _label)
          (else
            (`KismetSystemLibrary.PrintString` "BP_TestManager: No actor with BPI_TestScenario found on level")))))
    (else
      (`KismetSystemLibrary.PrintString` "ActiveConfig is None"))))

(event `StopRun`
  (bind (_global_runid _global_enablecsvprofiler _global_timelimittmax) (break `/Game/0-Main/Core/Structs/S_GlobalSettings` (`/Game/0-Main/Core/Configs/DA_TestConfig.Global` (`self.ActiveConfig`))))
  (set `self.bRunActive` false)
  (message `/Game/0-Main/Core/Interfaces/BPI_TestScenario.StopScenario` (`self.ScenarioActor`))
  (`KismetSystemLibrary.ExecuteConsoleCommand` "csvprofile stop" null)
  (if (> (`self.FPS_Count`) 0)
    (set `self.FPS_AVG` (/ (`self.FPS_Sum`) (`self.FPS_Count`))))
  (if (> (`self.Frame_Count`) 0)
    (set `self.Frame_AVG` (/ (`self.Frame_Sum`) (`self.Frame_Count`))))
  (bind _getscenarioname (message `/Game/0-Main/Core/Interfaces/BPI_TestScenario.GetScenarioName` (`self.ScenarioActor`)))
  (bind _returnvalue (`GameplayStatics.GetCurrentLevelName` true))
  (`KismetSystemLibrary.PrintString` (`KismetStringLibrary.Concat_StrStr` "RUN_END;" (`KismetStringLibrary.Concat_StrStr` "RunID" _global_runid "j") (`KismetStringLibrary.Concat_StrStr` "Scenario" _getscenarioname ";") (`KismetStringLibrary.Concat_StrStr` "Map" _returnvalue ";") (`KismetStringLibrary.Concat_StrStr` "Tmax" (`KismetStringLibrary.Conv_DoubleToString` _global_timelimittmax) ";") (`KismetStringLibrary.Concat_StrStr` "FPSavg" (`KismetStringLibrary.Conv_DoubleToString` (`self.FPS_AVG`)) ";") (`KismetStringLibrary.Concat_StrStr` "FPSmin" (`KismetStringLibrary.Conv_DoubleToString` (`self.FPS_Min`)) ";") (`KismetStringLibrary.Concat_StrStr` "FPSmax" (`KismetStringLibrary.Conv_DoubleToString` (`self.FPS_Max`)) ";") (`KismetStringLibrary.Concat_StrStr` "FRAMEavg" (`KismetStringLibrary.Conv_DoubleToString` (`self.Frame_AVG`)) ";") (`KismetStringLibrary.Concat_StrStr` "FRAMEmin" (`KismetStringLibrary.Conv_DoubleToString` (`self.Frame_Min`)) ";") (`KismetStringLibrary.Concat_StrStr` "FRAMEmax" (`KismetStringLibrary.Conv_DoubleToString` (`self.Frame_Max`)) ";"))))

(event `self.ReceiveTick`
  (params (DeltaSeconds :type "Float (single-precision)"))
  (if (`self.bRunActive`)
    (set `self.FPS` (/ 1.0 DeltaSeconds))
    (set `self.FPS_Min` (`KismetMathLibrary.FMin` (`self.FPS`) (`self.FPS_Min`)))
    (set `self.FPS_Max` (`KismetMathLibrary.FMax` (`self.FPS`) (`self.FPS_Max`)))
    (set `self.FPS_Sum` (+ (`self.FPS_Sum`) (`self.FPS`)))
    (set `self.FPS_Count` (+ (`self.FPS_Count`) 1))
    (set `self.Frames` DeltaSeconds)
    (set `self.Frame_Min` (`KismetMathLibrary.FMin` (`self.Frame_Min`) (`self.Frames`)))
    (set `self.Frame_Max` (`KismetMathLibrary.FMax` (`self.Frame_Max`) (`self.Frames`)))
    (set `self.Frame_Sum` (+ (`self.Frame_Sum`) (`self.Frames`)))
    (set `self.Frame_Count` (+ (`self.Frame_Count`) 1))))

(fn `UserConstructionScript`)